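; Tree trap actor that continuously spins its static mesh around the local roll axis.
; Each Tick checks RotBackward, then RotForward, sets RotationSpeed to a fixed positive or negative value and calls the matching rotate function.
; Both functions apply the same delta-time-scaled local rotation without sweep, so only the speed's sign sets direction.
; The file never sets either flag, and BeginPlay and overlap events are empty.
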(event EventBeginPlay)

(event Collision|EventActorBeginOverlap
  (params (OtherActor :type Actor%20Object%20Reference)))

(event EventTick
  (params (DeltaSeconds :type Float%20%28single-precision%29))
  (if (Variables|Default|GetRotBackward)
    (Variables|Default|SetRotationSpeed 2e+01)
    (CallFunction|RotateBackwards DeltaSeconds)
    (elif (Variables|Default|GetRotForward)
      (Variables|Default|SetRotationSpeed -2e+01)
      (CallFunction|RotateForward DeltaSeconds))))

(fn ConstructionScript)

(fn RotateForward
  (params (Time :type Float%20%28single-precision%29))
  (Transformation|AddLocalRotation (Variables|Default|GetStaticMesh) (* (Math|Rotator|MakeRotator (Variables|Default|GetRotationSpeed) 0.0 0.0) Time) false false))

(fn RotateBackwards
  (params (Time :type Float%20%28single-precision%29))
  (Transformation|AddLocalRotation (Variables|Default|GetStaticMesh) (* (Math|Rotator|MakeRotator (Variables|Default|GetRotationSpeed) 0.0 0.0) Time) false false))