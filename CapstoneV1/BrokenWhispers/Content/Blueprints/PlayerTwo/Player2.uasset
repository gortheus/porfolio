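; Player2 Blueprint that slides its Cube2 component to a target position and counts elapsed play time.
; On BeginPlay it records a start time and eases Cube2 out to Cube's relative location with a timed MoveComponentTo.
; Tick accumulates world delta seconds and stores the truncated difference from the start time as whole elapsed seconds.
; The overlap event is empty, and the player-index lookup and debug print are unconnected.
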(event EventBeginPlay
  (bind _output_get (Variables|Default|SetStart%20Time (stale EventTick DeltaSeconds)))
  (Components|MoveComponentTo (Variables|Default|GetCube2) (Variables|/Script/Engine.SceneComponent|GetRelativeLocation (Variables|Default|GetCube)) "0, 0, 0" true false 1e+01 false))

(event Collision|EventActorBeginOverlap
  (params (OtherActor :type Actor%20Object%20Reference)))

(event EventTick
  (params (DeltaSeconds :type Float%20%28single-precision%29))
  (bind _output_get (Variables|Default|SetTime%20Level (+ (Utilities|Time|GetWorldDeltaSeconds) (Variables|Default|GetTime%20Level))))
  (Variables|Default|SetEllapsed%20TIme (Math|Float|Truncate (- _output_get (stale EventBeginPlay _output_get)))))

(fn ConstructionScript)