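; OscReciever is an actor that handles two-way OSC messaging with a remote sender, including a /door value stored as DoorState.
; The first message received registers the sender's IP on port 33001 as a send target and starts a looping timer.
; The timer periodically sends queued messages as one bundle and clears the queue, which AddOSC_Message fills.
; Later messages are routed by address, with unknown ones printed.
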(event Custom|OSC_Run
  (bind _oscmessages (Variables|Default|GetOSCMessages))
  ;[1 1 1] Send OSC Messages
  (if (> (Utilities|Array|Length _oscmessages) 0)
    (Class|OscFunctionLibrary|SendOscBundle _oscmessages -1)
    (Utilities|Array|Clear _oscmessages)))

(event Custom|OSC_Rx
  (params (Address :type Name%20%28by%20ref%29) (Data :type Array%20of%20Osc%20Data%20Elem%20Struct%20Structures) (SenderIp :type String))
  (if (Variables|Default|GetStarted_OSC)
    (switch string (Utilities|String|ToString(Name) Address)
      (:Default
        (Development|PrintString (Utilities|String|ToString(Text) (Utilities|Text|FormatText "Message with address: {addr}  from: {ip}" (Utilities|Text|ToText(Name) Address) (Utilities|Text|ToText(String) SenderIp)))))
      (:/door
        (Variables|Default|Setdoor_state (.Value (Class|OscFunctionLibrary|PopInt Data)))
        (Development|PrintString "Received door val")))
    (else
      ;[1 1 1] OSC Setup: Get Send Target
      (Class|OscFunctionLibrary|AddSendOscTarget (Utilities|String|ToString(Text) (Utilities|Text|FormatText "{ip}:33001" (Utilities|Text|ToText(String) SenderIp))))
      (CallFunction|StartOSC)
      (Variables|Default|SetStarted_OSC true)
      (Development|PrintString "GotIP"))))

(event Custom|AddOSC_Message
  (params (TargetAddress :type String) (OSC_Data :type Array%20of%20Osc%20Data%20Elem%20Struct%20Structures))
  ;[1 1 1] Add OSC Message
  (Utilities|Array|Add (Variables|Default|GetOSCMessages) (Utilities|Struct|MakeOscMessageStruct (Utilities|String|StringToName TargetAddress) OSC_Data)))

(event Custom|StartOSC
  ;[1 1 1] Send OSC Messages
  (Utilities|Time|SetTimerbyEvent (delegate Custom|OSC_Run) 0.05 true))

(event EventBeginPlay
  (EventDispatchers|BindEventtoOnOscReceived (Variables|Default|GetOscReceiver) (delegate Custom|OSC_Rx)))

(event Collision|EventActorBeginOverlap
  (params (OtherActor :type Actor%20Object%20Reference)))

(event EventTick
  (params (DeltaSeconds :type Float%20%28single-precision%29)))

(fn ConstructionScript)